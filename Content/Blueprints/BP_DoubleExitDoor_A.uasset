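; BP_DoubleExitDoor_A is a platformer exit door that ends the level once the game mode's objective is complete.
; On BeginPlay it caches BP_Platformer_GM, then checks that flag when its collision is overlapped.
; If set, it swaps to the open sprite and disables its collision.
; For BP_RobotPlayer_C, it then stops movement, calls FinishLevel on the player HUD and opens NextLevel after a short delay.
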(event OnComponentBeginOverlap(Collision)
  (params (OverlappedComponent :type Primitive%20Component%20Object%20Reference) (OtherActor :type Actor%20Object%20Reference) (OtherComp :type Primitive%20Component%20Object%20Reference) (OtherBodyIndex :type Integer) (bFromSweep :type Boolean) (SweepResult :type Hit%20Result%20Structure%20%28by%20ref%29))
  (bind _gamemode (Variables|Default|GetGameMode))
  (bind _isobjectivecomplete (Variables|/Game/Blueprints/Player/BP_Platformer_GM.BP_Platformer_GM_C|GetisObjectiveComplete _gamemode))
  (bind _returnvalue (== _isobjectivecomplete true))
  ;[0.3728 1 0.4944] Level End Logic
  ;[0.4012 1 0.6002] Door Open Code (Sprite)
  (if _returnvalue
    (Rendering|Components|Sprite|SetSprite (Variables|Default|GetDoorSprite) "/Game/Sprites/DoubleDoor/S_DoubleDoor_Open.S_DoubleDoor_Open")
    (Collision|SetCollisionEnabled (Variables|Default|GetCollision) "NoCollision")
    (bind _asbp_robot_player_c (Utilities|Casting|CastToBP_RobotPlayer_C OtherActor))
    (Pawn|Components|CharacterMovement|DisableMovement (Variables|/Script/Engine.Character|GetCharacterMovement _asbp_robot_player_c))
    (if _returnvalue
      (Default|FinishLevel (Variables|/Game/Blueprints/Player/BP_RobotPlayer_C.BP_RobotPlayer_C_C|GetPlayerHUD _asbp_robot_player_c))
      (Utilities|FlowControl|Delay 2.0)
      (Game|OpenLevel(byObjectReference) (Variables|Default|GetNextLevel)))))

(event EventBeginPlay
  ;[1 0.4828 0.6449] Allocate Game Mode
  (bind _asbp_platformer_gm (Utilities|Casting|CastToBP_Platformer_GM (Game|GetGameMode)))
  (Variables|Default|SetGameMode _asbp_platformer_gm))

(fn ConstructionScript)