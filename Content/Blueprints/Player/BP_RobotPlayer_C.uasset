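; Paper2D robot player character that moves along X, jumps, and restarts the level on death.
; BeginPlay binds an Enhanced Input mapping context and creates the HUD; movement input also turns the controller to face left or right.
; Tick picks idle, walk, jump or die flipbooks from velocity and state flags.
; PlayerDie ends the level on the HUD, waits out the death flipbook, then reloads the current level.
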(event Custom|AnimationUpdateHandler
  (bind _f_playerstate (Variables|Default|GetF_PlayerState))
  ;[0.9524 1 0.5568] Animation Handler
  (if (== (Variables|Default|GetisPlayerDead) true)
    (Sprite|SetFlipbook (Variables|Default|GetF_PlayerState) "/Game/Sprites/Robot/Flipbook/F_Robot_Die.F_Robot_Die")
    (elif (== (Variables|Default|GetisJumping) false)
      (if (== (.z (Transformation|GetVelocity)) 0.0)
        (Sprite|SetFlipbook _f_playerstate (select (> (Math|Vector|VectorLength (Transformation|GetVelocity)) 0.0) "/Game/Sprites/Robot/Flipbook/F_Robot_Walk.F_Robot_Walk" "/Game/Sprites/Robot/Flipbook/F_Robot_Idle.F_Robot_Idle"))
        (else
          (Sprite|SetFlipbook _f_playerstate "/Game/Sprites/Robot/Flipbook/F_Robot_Jump.F_Robot_Jump"))))))

(event Custom|PlayerDie
  ;[1 0 0] Kill the Player (reset the level)
  (Variables|Default|SetisPlayerDead true)
  (CallFunction|AnimationUpdateHandler)
  (bind _animation_time (CallFunction|GetAnimationLength))
  (Default|EndLevel (Variables|Default|GetPlayerHUD))
  (Utilities|FlowControl|Delay _animation_time)
  (bind _returnvalue (Game|GetCurrentLevelName true))
  (Game|OpenLevel(byName) (Utilities|String|StringToName _returnvalue)))

(event Input|EnhancedActionEvents|EnhancedInputActionIA_Movement_Robot
  (params (ActionValue :type Float%20%28double-precision%29) (ElapsedSeconds :type Float%20%28double-precision%29) (TriggeredSeconds :type Float%20%28double-precision%29) (InputAction :type Input%20Action%20Object%20Reference :default "/Game/Blueprints/Player/Input/IA_Movement_Robot.IA_Movement_Robot"))
  (bind _playercontroller (Variables|Default|GetPlayerController))
  ;[1 0.749 0.6377] Player Movement
  (if (!= (Variables|Default|GetisPlayerDead) true)
    (Pawn|Input|AddMovementInput "1.000000,0.000000,0.000000" ActionValue false)
    (Math|Float|CompareFloat ActionValue 0.0
      (:>
        (Pawn|SetControlRotation _playercontroller (Math|Rotator|MakeRotator 0.0 0.0 0.0)))
      (:<
        (Pawn|SetControlRotation _playercontroller (Math|Rotator|MakeRotator 0.0 0.0 1.8e+02))))))

(event Input|EnhancedActionEvents|EnhancedInputActionIA_Jump_Robot
  (params (ActionValue :type Boolean) (ElapsedSeconds :type Float%20%28double-precision%29) (TriggeredSeconds :type Float%20%28double-precision%29) (InputAction :type Input%20Action%20Object%20Reference :default "/Game/Blueprints/Player/Input/IA_Jump_Robot.IA_Jump_Robot"))
  (bind _f_playerstate (Variables|Default|GetF_PlayerState))
  ;[1 0.749 0.6377] Player Movement
  (if (!= (Variables|Default|GetisPlayerDead) true)
    (Variables|Default|SetisJumping true)
    (Character|Jump (Game|GetPlayerCharacter 0))
    (Sprite|SetFlipbook _f_playerstate "/Game/Sprites/Robot/Flipbook/F_Robot_Jump.F_Robot_Jump")
    (Utilities|FlowControl|Delay 0.7)
    (Sprite|SetFlipbook _f_playerstate "/Game/Sprites/Robot/Flipbook/F_Robot_Walk.F_Robot_Walk")
    (Variables|Default|SetisJumping false)))

(event EventBeginPlay
  (bind _returnvalue (Game|GetPlayerController 0))
  ;[1 0.3542 0.3542] Allocate Input mapping context (start)
  (Variables|Default|SetPlayerController (Pawn|GetController))
  (Variables|Default|SetisPlayerDead false)
  (CallFunction|BindInputMapping)
  (bind _returnvalue_2 (UserInterface|CreateWidget "/Game/Blueprints/Player/BP_Player_UI.BP_Player_UI_C" _returnvalue))
  (UserInterface|Viewport|AddtoViewport _returnvalue_2 0)
  (Variables|Default|SetPlayerHUD _returnvalue_2)
  (Input|SetInputModeGameandUI _returnvalue 0 "DoNotLock" true false))

(event EventTick
  (params (DeltaSeconds :type Float%20%28single-precision%29))
  ;[0.4485 1 0.3441] Update()
  (CallFunction|AnimationUpdateHandler))

(fn ConstructionScript)

(fn GetAnimationLength
  (bind _f_playerstate (Variables|Default|GetF_PlayerState))
  (return (- (/ (Class|PaperFlipbookComponent|GetFlipbookLengthinFrames _f_playerstate) (Class|PaperFlipbookComponent|GetFlipbookFramerate _f_playerstate)) 0.1)))

(fn BindInputMapping
  (bind _asplayer_controller (Utilities|Casting|CastToPlayerController (Pawn|GetController)))
  (Input|AddMappingContext (PlayerController|LocalPlayerSubsystems|GetEnhancedInputLocalPlayerSubsystem _asplayer_controller) "/Game/Blueprints/Player/Input/IMC_RobotPlayer.IMC_RobotPlayer" 0 "(bIgnoreAllPressedKeysUntilRelease=True,bForceImmediately=False,bNotifyUserSettings=False)"))