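; BP_ElectroNode_A is an electrified hazard node that kills the robot player on overlap while it is active.
; A kill plays a hit flipbook, waits for nearly its full length, then switches to the off flipbook without clearing the Active flag.
; The ElectroNodePowerOff event disarms the node by clearing Active and showing the off flipbook.
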(event OnComponentBeginOverlap(Collider)
  (params (OverlappedComponent :type Primitive%20Component%20Object%20Reference) (OtherActor :type Actor%20Object%20Reference) (OtherComp :type Primitive%20Component%20Object%20Reference) (OtherBodyIndex :type Integer) (bFromSweep :type Boolean) (SweepResult :type Hit%20Result%20Structure%20%28by%20ref%29))
  (bind _flipbookstate (Variables|Default|GetFlipbookState))
  (bind _asbp_robot_player_c (Utilities|Casting|CastToBP_RobotPlayer_C OtherActor))
  (if (== (Variables|Default|GetActive) true)
    (Default|PlayerDie _asbp_robot_player_c)
    (Sprite|SetFlipbook _flipbookstate "/Game/Sprites/ElectroNode/Flipbook/F_ElectroNode_Hit.F_ElectroNode_Hit")
    (Utilities|FlowControl|Delay (- (/ (Class|PaperFlipbookComponent|GetFlipbookLengthinFrames _flipbookstate) (Class|PaperFlipbookComponent|GetFlipbookFramerate _flipbookstate)) 0.1))
    (Sprite|SetFlipbook (Variables|Default|GetFlipbookState) "/Game/Sprites/ElectroNode/Flipbook/F_ElectroNode_Off.F_ElectroNode_Off")))

(event Custom|ElectroNode%20Power%20Off
  (Variables|Default|SetActive false)
  (Sprite|SetFlipbook (Variables|Default|GetFlipbookState) "/Game/Sprites/ElectroNode/Flipbook/F_ElectroNode_Off.F_ElectroNode_Off"))

(fn ConstructionScript)